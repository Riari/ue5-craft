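; World pickup actor for an equipment item, collected when the player character overlaps its capsule.
; On BeginPlay it spawns the item actor from its ItemDefinition, binds it to a looping pickup Level Sequence, and tints the Niagara effect using a rarity colour data table.
; On overlap it passes the item to B_PlayerCharacter, plays a sound, then destroys both the item and itself.
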(event `self.ReceiveBeginPlay`
  (bind _itemdefinition (`self.ItemDefinition`))
  (`|ExecutionSequence`
    (:`then_0`
      (bind _returnvalue (`|SpawnActorFromClass` (`ItemDefinition.EquipmentItemClass` _itemdefinition) (`self.GetTransform`) "Undefined" "MultiplyWithRoot" null null))
      (set `self.Item` _returnvalue)
      (bind (_outactor _returnvalue_2) (`LevelSequencePlayer.CreateLevelSequencePlayer` "/Game/Actors/LS_Item_PickUp.LS_Item_PickUp"))
      (`LevelSequenceActor.AddBinding` _outactor (`|GetSequenceBinding` null) _returnvalue false)
      (`MovieSceneSequencePlayer.PlayLooping` _returnvalue_2 -1)
      (bind _returnvalue_3 (`|GetDataTableRow` (`self.ItemRarityColours`) (`KismetStringLibrary.Conv_StringToName` (`|GetEnumeratorNameAsString` (`ItemDefinition.Rarity` _itemdefinition))))
        (:`then`
          (`NiagaraComponent.SetVariableLinearColor` (`self.NS_Item_PickUp`) "Color" (`.Colour` (break `ItemRarityColourTableRow` _returnvalue_3))))))
    (:`then_1`
      (add `PrimitiveComponent.OnComponentBeginOverlap` (`self.CollectionCapsule`) (delegate `OnOverlap`)))))

(event `OnOverlap`
  (params (OverlappedComponent :type "PrimitiveComponent Object Reference") (OtherActor :type "Actor Object Reference") (OtherComp :type "PrimitiveComponent Object Reference") (OtherBodyIndex :type Integer) (bFromSweep :type Boolean) (SweepResult :type "HitResult Structure (by ref)"))
  (bind _item (`self.Item`))
  (bind _asb_player_character (cast `/Game/Actors/Characters/B_PlayerCharacter` OtherActor))
  (`CraftCharacter.OnItemPickUp` _asb_player_character _item)
  (`GameplayStatics.SpawnSoundAtLocation` "/Game/Sounds/ItemPickUp.ItemPickUp" (`KismetMathLibrary.TransformLocation` (`self.GetTransform`)) (struct) 1.0 1.0 0.0 null null)
  (`self.K2_DestroyActor` _item)
  (`self.K2_DestroyActor`))

(fn `UserConstructionScript`)